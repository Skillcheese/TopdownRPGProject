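; Player Ice Cascade skill actor that erupts a forward-spreading field of ice particle bursts and hits pawns caught in it.
; On BeginPlay, a Cascade event re-calls itself after short delays until its count runs out.
; Each wave spawns more randomized emitters in a wider band, with forward steps shrinking as GetAlpha progress rises.
; Every emitter runs a sphere trace that ignores the instigator and passes hits to ActorHit.
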(event Custom|Cascade
  (params (Num :type Integer))
  (bind _alpha (CallFunction|GetAlpha))
  (bind _returnvalue (Math|Float|Lerp 2.5e+02 7.5e+02 _alpha))
  (Math|Integer|CompareInt Num
    (:>
      (Math|Integer|IncrementInt (Variables|Default|GetIndex)
        (:%20%20
          (for _index (range 0 (/ (Variables|Default|GetIndex) 2))
            (bind _returnvalue_2 (Effects|SpawnEmitteratLocation (select (Math|Random|RandomBool) "/Game/Abilities/Player/Skills/IceCascade/IceCascade1.IceCascade1" "/Game/Abilities/Player/Skills/IceCascade/IceCascade2.IceCascade2") (- (+ (* (Transformation|GetActorForwardVector) (+ (Variables|Default|GetCurrent) (Math|Random|RandomFloatinRange -2e+01 2e+01))) (Transformation|GetActorLocation) (* (Transformation|GetActorRightVector) (Math|Random|RandomFloatinRange (* _returnvalue -1.0) _returnvalue))) "0, 0,133.000000")))
            (Effects|Components|ParticleSystem|SetVectorParameter _returnvalue_2 "Rotation" (Math|Vector|MakeVector 0.0 (Math|Float|Lerp 0.0 -0.1 (CallFunction|GetAlpha)) (/ (+ (Math|Random|RandomFloatinRange -15.0 15.0) (.yaw (Transformation|GetActorRotation))) 3.6e+02)))
            (Effects|Components|ParticleSystem|SetVectorParameter _returnvalue_2 "Size" "0.600000,0.600000,0.600000")
            (bind _outhits (Collision|MultiSphereTraceForObjects (Transformation|GetWorldLocation _returnvalue_2) (Transformation|GetWorldLocation _returnvalue_2) 1.5e+02 (Utilities|Array|MakeArray "ObjectTypeQuery3") false (Utilities|Array|MakeArray (Variables|Default|GetInstigator)) "None"))
            (for _array_element _outhits
              (CallFunction|ActorHit (.hitactor _array_element))))
          (Variables|Default|SetCurrent (+ (Variables|Default|GetCurrent) (Math|Float|Lerp (Math|Random|RandomFloatinRange 1e+02 2e+02) (Math|Random|RandomFloatinRange 15.0 3e+01) (CallFunction|GetAlpha))))
          (Utilities|FlowControl|Delay 0.03)
          (CallFunction|Cascade (- Num 1)))))))

(event EventBeginPlay
  (|CallParentFunction)
  (CallFunction|Cascade (Variables|Default|GetNumCascade))
  (Variables|Default|SetIndex 0))

(event EventTick
  (params (DeltaSeconds :type Float%20%28single-precision%29)))

(fn ConstructionScript
  (|CallParentFunction))

(fn GetAlpha
  (return (/ (Math|Conversions|ToFloat(Integer) (Variables|Default|GetIndex)) (Math|Conversions|ToFloat(Integer) (Variables|Default|GetNumCascade)))))