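; Deprecated player skill ability that warps the avatar instantly forward along its facing direction.
; DoAction spawns the warp particle and applies the container's effect, teleports the avatar, then repeats both at the destination.
; A raised sphere trace against WorldStatic sets the destination: just off the hit surface, or full range if clear.
; The move is unswept, so only that trace checks for obstacles.
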(event EventDoAction
  (params (ContainerTag :type Gameplay%20Tag%20Structure) (EventData :type Gameplay%20Event%20Data%20Structure%20%28by%20ref%29))
  (bind _returnvalue (Ability|GetAvatarActorfromActorInfo))
  (bind _returnvalue_2 (Transformation|GetActorLocation _returnvalue))
  (bind _returnvalue_3 (Transformation|GetActorForwardVector _returnvalue))
  (bind _returnvalue_4 (* _returnvalue_3 1e+03))
  (bind _returnvalue_5 (+ _returnvalue_2 "0.000000, 0,50.000000"))
  (bind _returnvalue_6 (+ _returnvalue_5 _returnvalue_4))
  (Utilities|FlowControl|Sequence
    (:then_0
      (Effects|SpawnEmitteratLocation "/Game/Abilities/Player/Deprecated/Skills/Warp/P_Warp.P_Warp" _returnvalue_2 (Transformation|GetActorRotation _returnvalue) :!label _label)
      (CallFunction|ApplyEffect ContainerTag EventData))
    (:then_1
      (bind (_outhit _returnvalue_7) (Collision|SphereTraceForObjects _returnvalue_5 _returnvalue_6 35.0 (Utilities|Array|MakeArray "ObjectTypeQuery1") false (Utilities|Array|MakeArray _returnvalue) "None"))
      (if _returnvalue_7
        (Transformation|SetActorLocation _returnvalue (+ (.location _outhit) (* (.normal _outhit) 3e+01)) false false)
        (else
          (Transformation|SetActorLocation _returnvalue (- _returnvalue_6 "0, 0,50.000000") false false))))
    (:then_2
      (goto _label))))