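; Base gameplay ability that fires one or more projectiles in an evenly spaced arc from the avatar's socket or location.
; Activation checks cost and cooldown, committing each immediately or deferring it until the montage event.
; Montage events, limited to one UseSkill outside footstep mode, build an effect container spec passed to each projectile if it has effects.
; Player characters aim yaw at the cursor hit; other avatars use their own rotation.
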(event Ability|EventActivateAbility
  (bind _returnvalue (Class|GameplayAbility|CheckAbilityCost))
  (if _returnvalue
    (bind _returnvalue_2 (Class|GameplayAbility|CheckAbilityCooldown))
    (if _returnvalue_2
      (if (Variables|Default|GetDelayedCost)
        (if (Variables|Default|GetDelayedCooldown) :!label _label
          (if (Variables|Default|GetIsFootstep) :!label _label_2
            (bind (_asynctaskproxy _eventtag _eventdata) (|PlayMontageandWaitforEvent "None" 0 "(GameplayTags=((TagName=\"Event.Montage\")))" 1.0 "None" true 1.0)
              (:EventReceived
                (Utilities|DoCommits)
                (bind _returnvalue_3 (Class|RPGGameplayAbility|MakeEffectContainerSpec _eventtag _eventdata (CallFunction|GetGALevel (Utilities|GetClass self))))
                (Utilities|SpawnProjectile(s) _returnvalue_3)))
            (else
              (bind (_asynctaskproxy_2 _eventtag_2 _eventdata_2) (|PlayMontageandWaitforEvent "None" (Variables|Default|GetMontageToPlay) "(GameplayTags=((TagName=\"Event.Montage\")))" (Variables|Default|GetMontagePlayRate) "None" true 1.0)
                (:OnBlendOut
                  (Ability|EndAbility :!label _label_3)
                  (goto _label_4 Reset))
                (:OnInterrupted
                  (goto _label_3))
                (:OnCancelled
                  (goto _label_3))
                (:EventReceived
                  (Utilities|FlowControl|DoOnce false :!label _label_4
                    (:Completed
                      (if (== _eventtag_2 "(TagName=\"Event.Montage.Shared.UseSkill\")")
                        (Utilities|DoCommits)
                        (bind _returnvalue_4 (Class|RPGGameplayAbility|MakeEffectContainerSpec _eventtag_2 _eventdata_2 (CallFunction|GetGALevel (Utilities|GetClass self)))) ; Make our container spec for later usage
                        (Utilities|SpawnProjectile(s) _returnvalue_4))))))))
          (else
            (bind _returnvalue_5 (Ability|CommitAbilityCooldown true))
            (if _returnvalue_5
              (goto _label_2))))
        (else
          (bind _returnvalue_6 (Ability|CommitAbilityCost true))
          (if _returnvalue_6
            (goto _label)))))))