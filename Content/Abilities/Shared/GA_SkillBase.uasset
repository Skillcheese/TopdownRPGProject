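; Base gameplay ability for skills that plays a montage and applies effect containers from its gameplay events.
; InitialChecks tests cost and cooldown, committing each immediately unless flagged as delayed; FinalChecks commits delayed ones when the montage event arrives.
; A DoOnce lets only the first Event.Montage event reach DoAction, which applies the tagged container at the class's ability level.
; Blend out, interruption or cancellation ends the ability.
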(event Custom|DoAction
  (params (ContainerTag :type Gameplay%20Tag%20Structure) (EventData :type Gameplay%20Event%20Data%20Structure%20%28by%20ref%29))
  (CallFunction|ApplyEffect ContainerTag EventData))

(event Custom|PlayMontage
  (bind (_asynctaskproxy _eventtag _eventdata) (|PlayMontageandWaitforEvent "None" (Variables|Default|GetMontageToPlay) "(GameplayTags=((TagName=\"Event.Montage\")))" (Variables|Default|GetSpeed) (Variables|Default|GetStartSectionOverride) true 1.0) ; Wait for one of the triggering event tags
    (:OnBlendOut
      (Ability|EndAbility :!label _label)
      (goto _label_2 Reset))
    (:OnInterrupted
      (goto _label))
    (:OnCancelled
      (goto _label))
    (:EventReceived
      (Utilities|FlowControl|DoOnce false :!label _label_2
        (:Completed
          (Utilities|FinalChecks)
          (CallFunction|DoAction _eventtag _eventdata))))))

(event Custom|ApplyEffect
  (params (ContainerTag :type Gameplay%20Tag%20Structure) (EventData :type Gameplay%20Event%20Data%20Structure%20%28by%20ref%29))
  (Class|RPGGameplayAbility|ApplyEffectContainer ContainerTag EventData (CallFunction|GetGALevel (Utilities|GetClass self))) ; Builds an immediately applies an effect container
)

(event Ability|EventActivateAbility
  (Utilities|InitialChecks)
  (CallFunction|PlayMontage))