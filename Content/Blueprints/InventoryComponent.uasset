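; Grid inventory component that stores multi-cell items in a map keyed by each item's top-left slot.
; Adding an item first merges it into a matching stack, otherwise tries each unoccupied slot computed from stored item footprints.
; Placement checks bounds and overlap, optionally swapping out a colliding item, and calls UpdateItem to report changes.
; Grid bounds depend on a Size setting, though slot enumeration only handles the player inventory.
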(fn GetAllSlots
  (Utilities|FlowControl|Sequence
    (:then_0
      (switch Utilities|FlowControl|Switch|SwitchonInventorySizes (Variables|Default|GetSize)
        (:NewEnumerator0
          (for _index (range 0 9)
            (for _index_2 (range 0 7)
              (Utilities|Array|AddUnique (LocalVariables|GetR) (Utilities|Struct|MakeIntPoint _index _index_2)))))))
    (:then_1
      (return (LocalVariables|GetR)))))

(fn GetAllUnoccupiedSlots
  (bind _inventoryitems (Variables|Default|GetInventoryItems))
  (bind _slots (CallFunction|GetAllSlots))
  (LocalVariables|SetR _slots)
  (bind _keys (Utilities|Map|Keys _inventoryitems))
  (for _array_element _keys
    (bind _slots_2 (CallFunction|GetSlotsOccupiedbyItem _array_element (.Value (Utilities|Map|Find _inventoryitems _array_element))))
    (for _array_element_2 _slots_2
      (Utilities|Array|RemoveItem (LocalVariables|GetR) _array_element_2)))
  (return (LocalVariables|GetR)))

(fn GetSlotsOccupiedbyItem
  (params (Location :type Int%20Point%20Structure) (Item :type RPG%20Loot%20Object%20Reference))
  (bind (_x _y) (Utilities|Struct|BreakIntPoint Location))
  (bind (_width _height) (Class|RPGLoot|GetItemDimensions Item))
  (Utilities|FlowControl|Sequence
    (:then_0
      (for _index (range 0 (- _width 1))
        (for _index_2 (range 0 (- _height 1))
          (Utilities|Array|AddUnique (LocalVariables|GetR) (Utilities|Struct|MakeIntPoint (+ _x _index) (+ _y _index_2))))))
    (:then_1
      (return (LocalVariables|GetR)))))

(fn ContainsStackableItem?
  (params (Item :type RPG%20Loot%20Object%20Reference))
  (bind _basetype (Variables|/Script/ActionRPG.RPGLoot|GetBaseType Item))
  (bind _inventoryitems (Variables|Default|GetInventoryItems))
  (if (Variables|/Script/ActionRPG.RPGItem|GetStackable _basetype)
    (bind _keys (Utilities|Map|Keys _inventoryitems))
    (for _array_element _keys
      (if (and (Variables|/Script/ActionRPG.RPGItem|GetStackable (Variables|/Script/ActionRPG.RPGLoot|GetBaseType (.Value (Utilities|Map|Find _inventoryitems _array_element)))) (== (Variables|/Script/ActionRPG.RPGLoot|GetBaseType (.Value (Utilities|Map|Find _inventoryitems _array_element))) _basetype))
        (return true (.Value (Utilities|Map|Find _inventoryitems _array_element)) _array_element))))
  (return false 0 ""))

(fn IsSlotValid
  (params (Slot :type Int%20Point%20Structure))
  (bind _size (Variables|Default|GetSize))
  (return (and (and (>= (.x Slot) 0) (< (.x Slot) (Utilities|Select :Index _size :NewEnumerator0 10 :NewEnumerator1 10))) (and (>= (.y Slot) 0) (< (.y Slot) (Utilities|Select :Index _size :NewEnumerator0 8 :NewEnumerator1 8))))))

(fn AttemptAddItemtoSlot
  (params (Item :type RPG%20Loot%20Object%20Reference) (TopLeftCorner1 :type Int%20Point%20Structure) (ValidRemainingSlots1 :type Array%20of%20Int%20Point%20Structures) (AllowSwap :type Boolean))
  (bind _inventoryitems (Variables|Default|GetInventoryItems))
  (LocalVariables|SetValidRemainingSlots ValidRemainingSlots1)
  (LocalVariables|SetAddItem Item)
  (bind _output_get (LocalVariables|SetTopLeftCorner TopLeftCorner1))
  (bind _returnvalue (CallFunction|IsSlotValid (Utilities|Struct|MakeIntPoint (+ (.X (Utilities|Struct|BreakIntPoint _output_get)) (- (.Width (Class|RPGLoot|GetItemDimensions (LocalVariables|GetAddItem))) 1)) (+ (.Y (Utilities|Struct|BreakIntPoint _output_get)) (- (.Height (Class|RPGLoot|GetItemDimensions (LocalVariables|GetAddItem))) 1)))))
  (if _returnvalue
    (LocalVariables|SetFailed false)
    (if AllowSwap
      (for _index (range (.X (Utilities|Struct|BreakIntPoint (LocalVariables|GetTopLeftCorner))) (+ (- (.Width (Class|RPGLoot|GetItemDimensions (LocalVariables|GetAddItem))) 1) (.X (Utilities|Struct|BreakIntPoint (LocalVariables|GetTopLeftCorner)))))
        (for _index_2 (range (.Y (Utilities|Struct|BreakIntPoint (LocalVariables|GetTopLeftCorner))) (+ (- (.Height (Class|RPGLoot|GetItemDimensions (LocalVariables|GetAddItem))) 1) (.Y (Utilities|Struct|BreakIntPoint (LocalVariables|GetTopLeftCorner)))))
          (if (not (Utilities|Array|ContainsItem (LocalVariables|GetValidRemainingSlots) (Utilities|Struct|MakeIntPoint _index _index_2)))
            (if (LocalVariables|GetFoundCollidingItem?)
              (return false (LocalVariables|GetAddItem) false)
              (else
                (LocalVariables|SetFoundCollidingItem? true)
                (bind _keys (Utilities|Map|Keys (Variables|Default|GetInventoryItems)))
                (bind _array_element (Utilities|Array|ForEachLoopwithBreak _keys :!label _label)
                  (:LoopBody
                    (bind _slots (CallFunction|GetSlotsOccupiedbyItem _array_element (.Value (Utilities|Map|Find (Variables|Default|GetInventoryItems) _array_element))))
                    (if (Utilities|Array|ContainsItem _slots (Utilities|Struct|MakeIntPoint _index _index_2))
                      (LocalVariables|SetFoundCollidingItem (.Value (Utilities|Map|Find (Variables|Default|GetInventoryItems) _array_element)))
                      (LocalVariables|SetFoundCollidingItemLocation _array_element)
                      (goto _label Break)))))))))
      (if (LocalVariables|GetFoundCollidingItem?)
        (Utilities|Map|Remove _inventoryitems (LocalVariables|GetFoundCollidingItemLocation))
        (Utilities|Map|Add _inventoryitems (LocalVariables|GetTopLeftCorner) (LocalVariables|GetAddItem))
        (Default|CallUpdateItem (LocalVariables|GetTopLeftCorner) (LocalVariables|GetAddItem) true)
        (return true (LocalVariables|GetFoundCollidingItem) true)
        (else
          ;[1 1 1] If we Succeed
          (Utilities|Map|Add (Variables|Default|GetInventoryItems) (LocalVariables|GetTopLeftCorner) (LocalVariables|GetAddItem) :!label _label_2)
          (Default|CallUpdateItem (LocalVariables|GetTopLeftCorner) (LocalVariables|GetAddItem) true)
          (return true 0 true)))
      (else
        (bind _index_3 (Utilities|FlowControl|ForLoopwithBreak (.X (Utilities|Struct|BreakIntPoint (LocalVariables|GetTopLeftCorner))) (+ (- (.Width (Class|RPGLoot|GetItemDimensions (LocalVariables|GetAddItem))) 1) (.X (Utilities|Struct|BreakIntPoint (LocalVariables|GetTopLeftCorner)))) :!label _label_3)
          (:LoopBody
            (for _index_4 (range (.Y (Utilities|Struct|BreakIntPoint (LocalVariables|GetTopLeftCorner))) (+ (- (.Height (Class|RPGLoot|GetItemDimensions (LocalVariables|GetAddItem))) 1) (.Y (Utilities|Struct|BreakIntPoint (LocalVariables|GetTopLeftCorner)))))
              (if (not (Utilities|Array|ContainsItem (LocalVariables|GetValidRemainingSlots) (Utilities|Struct|MakeIntPoint _index_3 _index_4)))
                (LocalVariables|SetFailed true)
                (goto _label_3 Break))))
          (:Completed
            (if (LocalVariables|GetFailed)
              ;[1 1 1] Another item exists and allow swap is false
              (return false 0 false)
              (else
                (goto _label_2)))))))
    (else
      ;[1 1 1] If The item would go outside the inventory
      (return false (LocalVariables|GetAddItem) false))))

(fn RemoveItem
  (params (Item :type RPG%20Loot%20Object%20Reference))
  (bind (_returnvalue _location _success) (CallFunction|FindItemLocation Item))
  (if _success
    (bind _returnvalue_2 (Utilities|Map|Remove (Variables|Default|GetInventoryItems) _location))
    (return _returnvalue_2)
    (else
      (return false))))

(fn FindItemLocation
  (params (Item :type RPG%20Loot%20Object%20Reference))
  (bind _inventoryitems (Variables|Default|GetInventoryItems))
  (bind _keys (Utilities|Map|Keys _inventoryitems))
  (for _array_element _keys
    (if (== (.Value (Utilities|Map|Find _inventoryitems _array_element)) Item)
      (return Item _array_element true)))
  (return 0 "" false))

(fn AddNewItemtoInventory
  (params (Item :type RPG%20Loot%20Object%20Reference))
  (bind _output_get (LocalVariables|SetAddItem Item))
  (bind (_returnvalue _returnitem_if_valid_ _slot) (CallFunction|ContainsStackableItem? _output_get))
  (if _returnvalue
    (Class|RPGLoot|UpdateItemCount _returnitem_if_valid_ (Class|RPGLoot|GetItemCount (LocalVariables|GetAddItem)))
    (Default|CallUpdateItem _slot _returnitem_if_valid_ false)
    (return 0 true)
    (else
      (bind _r1 (CallFunction|GetAllUnoccupiedSlots))
      (for _array_element _r1
        (bind (_successfullyadded _remainingitem_if_valid_ _donotupdate) (CallFunction|AttemptAddItemtoSlot (LocalVariables|GetAddItem) _array_element _r1 false))
        (if _successfullyadded
          (if _donotupdate
            _
            (else
              (Default|CallUpdateItem _array_element (LocalVariables|GetAddItem) true)))
          (return 0 true)))
      (return (LocalVariables|GetAddItem) false))))