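; Blueprint function library of global RPG helpers for items, souls currency and affix rolling.
; Item and soul functions forward to the game instance and player controller, adding affix updates, inventory saving and a gain effect.
; Affix rolls pick a random tier, skipping six, and a percentage, then interpolate within data table ranges; a reverse lookup derives tier from value.
; Others check gear types, find granted-ability levels and price salvage using recursive triangular sums.
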(fn CreateItem
  (params (BaseType :type RPG%20Item%20Object%20Reference) (ItemLevel :type Integer))
  (bind _returnvalue (Class|RPGGameInstanceBase|CreateItem (CallFunction|GetGameInstanceBP (LocalVariables|Get__WorldContext)) BaseType ItemLevel))
  (if (Math|Boolean|ORBoolean (.bSuccess (Utilities|Casting|CastToRPGSkillItem (Variables|/Script/ActionRPG.RPGLoot|GetBaseType _returnvalue))) (.bSuccess (Utilities|Casting|CastToRPGArmorItem (Variables|/Script/ActionRPG.RPGLoot|GetBaseType _returnvalue))) (.bSuccess (Utilities|Casting|CastToRPGWeaponItem (Variables|/Script/ActionRPG.RPGLoot|GetBaseType _returnvalue))))
    (Class|RPGPlayerControllerBase|UpdateItemAffixes (CallFunction|GetPlayerControllerBP (LocalVariables|Get__WorldContext)) _returnvalue (Variables|/Script/ActionRPG.RPGItem|GetBasePrefix (Variables|/Script/ActionRPG.RPGLoot|GetBaseType _returnvalue)) (Variables|/Script/ActionRPG.RPGItem|GetBaseSuffix (Variables|/Script/ActionRPG.RPGLoot|GetBaseType _returnvalue)) (Variables|/Script/ActionRPG.RPGItem|GetBaseImplicit (Variables|/Script/ActionRPG.RPGLoot|GetBaseType _returnvalue)) (Variables|/Script/ActionRPG.RPGItem|GetBaseEnchants (Variables|/Script/ActionRPG.RPGLoot|GetBaseType _returnvalue))))
  (return _returnvalue))

(fn AddSouls
  (params (Amount :type Integer))
  (bind ___worldcontext (LocalVariables|Get__WorldContext))
  (LocalVariables|SetOldAmount (Class|RPGPlayerControllerBase|GetSouls (CallFunction|GetPlayerControllerBP (LocalVariables|Get__WorldContext))))
  (bind (_count _returnvalue) (Class|RPGPlayerControllerBase|AddSouls (CallFunction|GetPlayerControllerBP (LocalVariables|Get__WorldContext)) Amount))
  (Default|CallOnSoulsUpdated (CallFunction|GetPlayerControllerBP ___worldcontext) _count)
  (Class|RPGPlayerControllerBase|SaveInventory (CallFunction|GetPlayerControllerBP (LocalVariables|Get__WorldContext)))
  (if (> _count (LocalVariables|GetOldAmount))
    (Default|PlayMaterialEffect (CallFunction|GetPlayerCharacterBP ___worldcontext) "(R=0.000000,G=1.000000,B=1.000000,A=1.000000)"))
  (return _count _returnvalue))

(fn IsGearType
  (params (Type :type RPG%20Item%20Object%20Reference))
  (bind _itemtype (Variables|/Script/ActionRPG.RPGItem|GetItemType Type))
  (Utilities|IsValid Type
    (:Is%20Valid
      (return (Math|Boolean|ORBoolean (== _itemtype "Armor") (== _itemtype "Boots") (== _itemtype "Chest") (== _itemtype "Gloves") (== _itemtype "Helmet") (== _itemtype "Jewelry") (== _itemtype "Weapon"))))
    (:Is%20Not%20Valid
      (return false))))

(fn IsGear
  (params (Loot :type RPG%20Loot%20Object%20Reference))
  (Utilities|IsValid Loot
    (:Is%20Valid
      (return (CallFunction|IsGearType (Variables|/Script/ActionRPG.RPGLoot|GetBaseType Loot) (LocalVariables|Get__WorldContext))))
    (:Is%20Not%20Valid
      (return false))))

(fn DetermineSalvageValue
  (params (Item :type RPG%20Loot%20Object%20Reference))
  (return (* (Variables|/Script/ActionRPG.RPGItem|GetPrice (Variables|/Script/ActionRPG.RPGLoot|GetBaseType Item)) (+ (CallFunction|GetAddtorial (- (Class|RPGLoot|GetItemLevel Item) 1) (LocalVariables|Get__WorldContext)) 1))))

(fn GetSouls
  (return (Class|RPGPlayerControllerBase|GetSouls (CallFunction|GetPlayerControllerBP (LocalVariables|Get__WorldContext)))))

(fn GetGALevel
  (params (Ability :type RPG%20Gameplay%20Ability%20Class%20Reference))
  (bind _values (Utilities|Map|Values (Variables|/Script/ActionRPG.InventoryComponentC|GetEquipement (Variables|/Game/Blueprints/BP_PlayerController.BP_PlayerController_C|GetInventoryComponent (CallFunction|GetPlayerControllerBP (LocalVariables|Get__WorldContext))))))
  (for _array_element _values
    (Utilities|IsValid _array_element
      (:Is%20Valid
        (Utilities|IsValid (Variables|/Script/ActionRPG.RPGLoot|GetBaseType _array_element)
          (:Is%20Valid
            (if (== (Variables|/Script/ActionRPG.RPGItem|GetGrantedAbility (Variables|/Script/ActionRPG.RPGLoot|GetBaseType _array_element)) Ability)
              (return (Utilities|Struct|BreakRPGItemData (Variables|/Script/ActionRPG.RPGLoot|GetData _array_element)))))))))
  (return -1))

(fn GetEnhancementValues
  (params (Item :type RPG%20Loot%20Object%20Reference))
  (return (* (Utilities|Struct|BreakRPGItemData (Variables|/Script/ActionRPG.RPGLoot|GetData Item)) (Variables|/Script/ActionRPG.RPGItem|GetPrice (Variables|/Script/ActionRPG.RPGLoot|GetBaseType Item)))))

(fn SoulsPurchaseGlobal
  (params (amount :type Integer))
  (bind (_count _returnvalue) (Default|MakeSoulsPurchase (CallFunction|GetPlayerControllerBP (LocalVariables|Get__WorldContext)) amount))
  (return _count _returnvalue))

(fn GetAddtorial
  (params (Num :type Integer))
  (Math|Integer|CompareInt Num
    (:>
      (return (+ Num (CallFunction|GetAddtorial (- Num 1) (LocalVariables|Get__WorldContext)))))
    (:==
      (return 0))))

(fn RollAffixTier/Value
  (params (LockTier%280%20Means%20No%29 :type Integer) (LockValue%280%20Means%20No%29 :type Integer))
  (LocalVariables|SetTier_ LockTier%280%20Means%20No%29)
  (LocalVariables|SetValuePercent_ LockValue%280%20Means%20No%29)
  (Utilities|FlowControl|Sequence
    (:then_0
      (Math|Integer|CompareInt (LocalVariables|GetTier_)
        (:==
          (bind _output_get (LocalVariables|SetTier_ (Math|Random|RandomIntegerinRange 1 6)))
          (Math|Integer|CompareInt _output_get 6
            (:==
              (LocalVariables|SetTier_ 7))))))
    (:then_1
      (Math|Integer|CompareInt (LocalVariables|GetValuePercent_)
        (:==
          (LocalVariables|SetValuePercent_ (Math|Random|RandomIntegerinRange 1 100)))))
    (:then_2
      (return (LocalVariables|GetTier_) (LocalVariables|GetValuePercent_)))))

(fn GetAffixFinalValue
  (params (Affix :type GE%20Affix%20Class%20Reference) (Tier :type Integer) (Value :type Integer))
  (bind _affixtable (LocalVariables|GetAffixTable))
  (LocalVariables|SetAffixType Affix)
  (LocalVariables|SetTier# Tier)
  (LocalVariables|SetValuePercent Value)
  (bind _outrownames (DataTable|GetDataTableRowNames _affixtable))
  (for _array_element _outrownames
    (bind _returnvalue (Utilities|GetDataTableRow _affixtable _array_element)
      (:then
        (if (== (LocalVariables|GetAffixType) (.AffixType (Utilities|Struct|BreakTierValueStruct _returnvalue)))
          (Math|Integer|CompareInt (LocalVariables|GetTier#) 1
            (:>
              (Math|Integer|CompareInt (LocalVariables|GetTier#) 2
                (:>
                  (Math|Integer|CompareInt (LocalVariables|GetTier#) 3
                    (:>
                      (Math|Integer|CompareInt (LocalVariables|GetTier#) 4
                        (:>
                          (Math|Integer|CompareInt (LocalVariables|GetTier#) 5
                            (:>
                              (Math|Integer|CompareInt (LocalVariables|GetTier#) 7
                                (:>
                                  (return -1))
                                (:==
                                  (LocalVariables|SetBaseValue (.Tier6Range (Utilities|Struct|BreakTierValueStruct _returnvalue)))
                                  (LocalVariables|SetMaxValue (.Tier7Range (Utilities|Struct|BreakTierValueStruct _returnvalue))))))
                            (:==
                              (LocalVariables|SetBaseValue (.Tier4Range (Utilities|Struct|BreakTierValueStruct _returnvalue)))
                              (LocalVariables|SetMaxValue (.Tier5Range (Utilities|Struct|BreakTierValueStruct _returnvalue))))))
                        (:==
                          (LocalVariables|SetBaseValue (.Tier3Range (Utilities|Struct|BreakTierValueStruct _returnvalue)))
                          (LocalVariables|SetMaxValue (.Tier4Range (Utilities|Struct|BreakTierValueStruct _returnvalue))))))
                    (:==
                      (LocalVariables|SetBaseValue (.Tier2Range (Utilities|Struct|BreakTierValueStruct _returnvalue)))
                      (LocalVariables|SetMaxValue (.Tier3Range (Utilities|Struct|BreakTierValueStruct _returnvalue))))))
                (:==
                  (LocalVariables|SetBaseValue (.Tier1Range (Utilities|Struct|BreakTierValueStruct _returnvalue)))
                  (LocalVariables|SetMaxValue (.Tier2Range (Utilities|Struct|BreakTierValueStruct _returnvalue))))))
            (:==
              (LocalVariables|SetBaseValue (- (.StartValue (Utilities|Struct|BreakTierValueStruct _returnvalue)) 1))
              (LocalVariables|SetMaxValue (.Tier1Range (Utilities|Struct|BreakTierValueStruct _returnvalue))))
            (:<
              (return -1)))
          (return (Math|Integer|Max(Integer) (+ (LocalVariables|GetBaseValue) (Math|Float|Round (* (Math|Conversions|ToFloat(Integer) (- (LocalVariables|GetMaxValue) (LocalVariables|GetBaseValue))) (/ (Math|Conversions|ToFloat(Integer) (LocalVariables|GetValuePercent)) 1e+02)))) (+ (LocalVariables|GetBaseValue) 1)))))))
  (return -1))

(fn GetAffixTier
  (params (Affix :type GE%20Affix%20Class%20Reference) (Value :type Integer))
  (bind _affixtable (LocalVariables|GetAffixTable))
  (LocalVariables|SetAffixType Affix)
  (LocalVariables|SetFinalValue Value)
  (bind _outrownames (DataTable|GetDataTableRowNames _affixtable))
  (for _array_element _outrownames
    (bind _returnvalue (Utilities|GetDataTableRow _affixtable _array_element)
      (:then
        (if (== (LocalVariables|GetAffixType) (.AffixType (Utilities|Struct|BreakTierValueStruct _returnvalue)))
          (bind _output_get (LocalVariables|SetCompareValue (.Tier1Range (Utilities|Struct|BreakTierValueStruct _returnvalue))))
          (Math|Integer|CompareInt (LocalVariables|GetFinalValue) _output_get
            (:>
              (bind _output_get_2 (LocalVariables|SetCompareValue (.Tier2Range (Utilities|Struct|BreakTierValueStruct _returnvalue))))
              (Math|Integer|CompareInt (LocalVariables|GetFinalValue) _output_get_2
                (:>
                  (bind _output_get_3 (LocalVariables|SetCompareValue (.Tier3Range (Utilities|Struct|BreakTierValueStruct _returnvalue))))
                  (Math|Integer|CompareInt (LocalVariables|GetFinalValue) _output_get_3
                    (:>
                      (bind _output_get_4 (LocalVariables|SetCompareValue (.Tier4Range (Utilities|Struct|BreakTierValueStruct _returnvalue))))
                      (Math|Integer|CompareInt (LocalVariables|GetFinalValue) _output_get_4
                        (:>
                          (bind _output_get_5 (LocalVariables|SetCompareValue (.Tier5Range (Utilities|Struct|BreakTierValueStruct _returnvalue))))
                          (Math|Integer|CompareInt (LocalVariables|GetFinalValue) _output_get_5
                            (:>
                              (return 7))
                            (:==
                              _)
                            (:<
                              _))
                          (return 5))
                        (:==
                          _)
                        (:<
                          _))
                      (return 4))
                    (:==
                      _)
                    (:<
                      _))
                  (return 3))
                (:==
                  _)
                (:<
                  _))
              (return 2))
            (:==
              _)
            (:<
              _))
          (return 1)))))
  (return -1))

(fn RollAffix
  (params (Affix :type GE%20Affix%20Class%20Reference))
  (bind ___worldcontext (LocalVariables|Get__WorldContext))
  (bind (_tier _valuepercent) (CallFunction|RollAffixTier/Value 0 0 ___worldcontext))
  (return Affix (CallFunction|GetAffixFinalValue Affix _tier _valuepercent ___worldcontext)))